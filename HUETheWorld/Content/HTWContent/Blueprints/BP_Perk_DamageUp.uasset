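; BP_Perk_DamageUp is a perk pickup that temporarily boosts a player character's damage, with its duration set on BeginPlay.
; ApplyPerkEffect sets the character's damage multiplier and makes the pickup inactive.
; RemovePerkEffect reactivates it rather than destroying it, and sets the multiplier to the character's BaseDamage.
; Tick spins the sphere around yaw at a frame-rate-independent speed; overlap and timer handling are not in this graph.
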(event `self.ReceiveBeginPlay`
  (set `self.PerkDuration` 5.0))

(event `self.ReceiveTick`
  (params (DeltaSeconds :type "Float (single-precision)"))
  (`SceneComponent.K2_AddLocalRotation` (`self.Sphere`) (* (`KismetMathLibrary.MakeRotator` 0.0 0.0 1.0) (* DeltaSeconds (`self.RotationSpeed`))) false false))

(fn `ApplyPerkEffect`
  (params (CharacterPlayer :type "/Game/HTWContent/Blueprints/BP_Character_Player Object Reference"))
  (`/Game/HTWContent/Blueprints/BP_Character_Player.SetDamageMultiplier` CharacterPlayer (`self.DamageMultiplier`))
  (`self.SetInactive`))

(fn `RemovePerkEffect`
  (params (CharacterPlayer :type "/Game/HTWContent/Blueprints/BP_Character_Player Object Reference"))
  (`self.SetActive`)
  (`/Game/HTWContent/Blueprints/BP_Character_Player.SetDamageMultiplier` CharacterPlayer (`/Game/HTWContent/Blueprints/BP_Character_Player.BaseDamage` CharacterPlayer)))

(fn `UserConstructionScript`)