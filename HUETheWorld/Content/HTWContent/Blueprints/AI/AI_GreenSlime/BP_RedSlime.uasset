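; Red slime enemy character that damages the player on overlap and only takes damage from bullets matching its colour.
; Bullet hits update a camera-facing health bar widget and set the player on the AI blackboard.
; Attack launches it forward.
; At zero health, Tick plays death animation and sound once, notifies the game mode, rolls a random power-up drop, then destroys it.
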(event `self.ReceiveBeginPlay`
  (bind _currenthealth (`self.CurrentHealth`))
  (bind _healthbarwidget (`self.HealthBarWidget`))
  ;[1 1 1] Set current health of enemy
  (set `self.CurrentHealth` (`self.StartingHealth`))
  ;[1 1 1] Save Health bar Widget as a Variable
  (bind _aswidget_enemy_health_bar (cast `/Game/HTWContent/Blueprints/WIDGET_EnemyHealthBar` (`WidgetComponent.GetUserWidgetObject` (`self.HealthBar`))))
  (set `self.HealthBarWidget` _aswidget_enemy_health_bar)
  ;[1 1 1] Set MaxHealth and CurrentHealth of Widget
  (set `/Game/HTWContent/Blueprints/WIDGET_EnemyHealthBar.EnemyMaxHealth` (`self.StartingHealth`) _healthbarwidget)
  (set `/Game/HTWContent/Blueprints/WIDGET_EnemyHealthBar.EnemyCurrentHealth` _currenthealth _healthbarwidget)
  ;[1 1 1] Set Widget HealthProgress to be correct
  (`/Game/HTWContent/Blueprints/WIDGET_EnemyHealthBar.UpdateHealth` _healthbarwidget _currenthealth)
  (`/Game/HTWContent/Blueprints/WIDGET_EnemyHealthBar.SetColourOfHealthBar` _healthbarwidget (make `Color` 0 0 255 255)))

(event `self.ReceiveTick`
  (params (DeltaSeconds :type "Float (single-precision)"))
  (bind _mesh (`self.Mesh`))
  ;[1 1 1] If current Health is lesser than 0, destroy
  (if (<= (`self.CurrentHealth`) 0)
    (`/Engine/EditorBlueprintResources/StandardMacros.DoOnce` false
      (:`Completed`
        (`SceneComponent.K2_SetWorldTransform` _mesh (`SceneComponent.K2_GetComponentToWorld` _mesh) false false)
        (set `self.AIControllerClass` "/Script/Engine.Controller")
        (`SkeletalMeshComponent.PlayAnimation` (`self.Mesh`) "/Game/HTWContent/Animations/Die_Slime_Anim.Die_Slime_Anim" false)
        (`GameplayStatics.PlaySoundAtLocation` "/Game/HTWContent/Audio/SW_RedSlimeDeath.SW_RedSlimeDeath" (0.0 0.0 0.0) (struct) 1.0 1.0 0.0 null null null)
        (`KismetSystemLibrary.Delay` 0.9)
        (bind _asbp_game_mode_htwcgame_mode (cast `/Game/HTWContent/Blueprints/BP_GameMode_HTWCGameMode` (`GameplayStatics.GetGameMode`)))
        (`/Game/HTWContent/Blueprints/BP_GameMode_HTWCGameMode.ReduceEnemies_Event` _asbp_game_mode_htwcgame_mode)
        (if (<= (`KismetMathLibrary.RandomFloatInRange` 0.0 1.0) (`/Game/HTWContent/Blueprints/BP_GameMode_HTWCGameMode.PowerUpChance` _asbp_game_mode_htwcgame_mode))
          (bind _powerups (`/Game/HTWContent/Blueprints/BP_GameMode_HTWCGameMode.PowerUps` _asbp_game_mode_htwcgame_mode))
          (`|SpawnActorFromClass` (`|GetArrayItem` _powerups (`KismetMathLibrary.RandomIntegerInRange` 0 (- (`KismetArrayLibrary.Array_Length` _powerups) 1))) (`KismetMathLibrary.Conv_VectorToTransform` (`self.K2_GetActorLocation` self)) "Undefined" "OverrideRootScale" null null))
        (`self.K2_DestroyActor`)))
    (else
      ;[1 1 1] Rotate HealthBar to face Player
      (`self.RotateHealthBarToPlayer`))))

(event `self.CapsuleComponent.OnComponentHit`
  (params (HitComponent :type "PrimitiveComponent Object Reference") (OtherActor :type "Actor Object Reference") (OtherComp :type "PrimitiveComponent Object Reference") (NormalImpulse :type "Vector Structure") (Hit :type "HitResult Structure (by ref)"))
  ;[1 1 1] Check if Enemy is Overlapped by Bullet
  (if (== (`GameplayStatics.GetObjectClass` OtherActor) "/Game/HTWContent/Blueprints/BP_Actor_Bullet.BP_Actor_Bullet_C")
    (bind _asbp_actor_bullet (cast `/Game/HTWContent/Blueprints/BP_Actor_Bullet` OtherActor))
    ;[1 1 1] Check if Bullet is same colour as Enemy
    (if (`|EnumEquality` (`/Game/HTWContent/Blueprints/BP_Actor_Bullet.BulletColor` _asbp_actor_bullet) (`self.EnemyColour`))
      ;[1 1 1] TakeDamage from the Bullet
      (`/Game/HTWContent/Blueprints/BP_Enemy.TakeDamage` (`/Game/HTWContent/Blueprints/BP_Actor_Bullet.BulletDamage` _asbp_actor_bullet))
      ;[1 1 1] Update HealthBar Widget
      (`/Game/HTWContent/Blueprints/WIDGET_EnemyHealthBar.UpdateHealth` (`self.HealthBarWidget`) (`self.CurrentHealth`)))
    (`self.K2_DestroyActor` _asbp_actor_bullet)))

(event `/Game/HTWContent/Blueprints/BP_Enemy.TakeDamage`
  (params (DamageTaken :type Integer))
  (set `self.CurrentHealth` (- (`self.CurrentHealth`) DamageTaken))
  (`self.SeekPlayer`))

(event `/Game/HTWContent/Blueprints/BP_Enemy.Attack`
  (`self.LaunchCharacter` (* (`self.GetActorForwardVector`) 6000.0) true true))

(event `self.ReceiveActorBeginOverlap`
  (params (OtherActor :type "Actor Object Reference"))
  (bind _asbp_character_player (cast `/Game/HTWContent/Blueprints/BP_Character_Player` OtherActor))
  (if (not (`/Game/HTWContent/Blueprints/BP_Character_Player.isInvulnerable` _asbp_character_player))
    (`/Game/HTWContent/Blueprints/BP_Character_Player.TakeDamage` _asbp_character_player 1)
    (`GameplayStatics.PlaySoundAtLocation` "/Game/HTWContent/Audio/SW_RedSlimeHit.SW_RedSlimeHit" (`self.K2_GetActorLocation` self) (struct) 1.0 1.0 0.0 null null null)
    (`GameplayStatics.PlaySoundAtLocation` "/Game/HTWContent/Audio/Character_Damaged.Character_Damaged" (`self.K2_GetActorLocation` _asbp_character_player) (struct) 1.0 1.0 0.0 null null null)
    (`/Game/HTWContent/Blueprints/BP_Character_Player.TriggerInvulnerabilityPeriod` _asbp_character_player)))

(event `SeekPlayer`
  (`BlackboardComponent.SetValueAsObject` (`AIBlueprintHelperLibrary.GetBlackboard` self) (`self.Player`) (`GameplayStatics.GetPlayerCharacter` 0)))

(fn `RotateHealthBarToPlayer`
  (bind _healthbar (`self.HealthBar`))
  (`SceneComponent.K2_SetWorldRotation` _healthbar (`KismetMathLibrary.FindLookAtRotation` (`SceneComponent.K2_GetComponentLocation` _healthbar) (`PlayerCameraManager.GetCameraLocation` (`GameplayStatics.GetPlayerCameraManager` 0))) false false))

(fn `UserConstructionScript`)