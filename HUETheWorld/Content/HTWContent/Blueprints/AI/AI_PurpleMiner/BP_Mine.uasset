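; BP_Mine is a mine actor, filed with the PurpleMiner AI, that explodes when the player character touches it.
; On overlap it spawns explosion particles and sound at its mesh, then deals 1 damage and starts an invulnerability period unless the player is already invulnerable.
; The mine destroys itself after detonating, or when its Lifespan delay from BeginPlay runs out.
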(event `self.ReceiveBeginPlay`
  (`KismetSystemLibrary.Delay` (`self.Lifespan`))
  (`self.K2_DestroyActor`))

(event `self.ReceiveActorBeginOverlap`
  (params (OtherActor :type "Actor Object Reference"))
  (bind _returnvalue (`SceneComponent.K2_GetComponentLocation` (`self.StaticMesh`)))
  (if (== OtherActor (`GameplayStatics.GetPlayerCharacter` 0))
    (`GameplayStatics.SpawnEmitterAtLocation` "/Game/StarterContent/Particles/P_Explosion.P_Explosion" _returnvalue (struct) (0.8 0.8 0.8))
    (`GameplayStatics.PlaySoundAtLocation` "/Game/StarterContent/Audio/Explosion02.Explosion02" _returnvalue (struct) 1.0 1.0 0.0 null null null)
    (bind _asbp_character_player (cast `/Game/HTWContent/Blueprints/BP_Character_Player` OtherActor))
    (if (not (`/Game/HTWContent/Blueprints/BP_Character_Player.isInvulnerable` _asbp_character_player))
      (`/Game/HTWContent/Blueprints/BP_Character_Player.TakeDamage` _asbp_character_player 1)
      (`GameplayStatics.PlaySoundAtLocation` "/Game/HTWContent/Audio/Character_Damaged.Character_Damaged" (`self.K2_GetActorLocation` _asbp_character_player) (struct) 1.0 1.0 0.0 null null null)
      (`/Game/HTWContent/Blueprints/BP_Character_Player.TriggerInvulnerabilityPeriod` _asbp_character_player))
    (`self.K2_DestroyActor`)))

(event `self.ReceiveTick`
  (params (DeltaSeconds :type "Float (single-precision)")))

(fn `UserConstructionScript`)