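; Blue cannon enemy that fires cannonballs and only takes damage from bullets matching its colour.
; An Attack event spawns a cannonball ahead of the Forward component, while mesh hits destroy any bullet and update the health bar widget on a match.
; Tick turns the health bar toward the player camera until health runs out.
; A timeline then tilts the mesh, with a death sound, GameMode enemy-count reduction and delayed destruction.
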(event `self.ReceiveBeginPlay`
  (bind _currenthealth (`self.CurrentHealth`))
  (bind _healthbarwidget (`self.HealthBarWidget`))
  ;[1 1 1] Set current health of Enemy
  (set `self.CurrentHealth` (`self.StartingHealth`))
  ;[1 1 1] Save Health bar Widget as a Variable
  (bind _aswidget_enemy_health_bar (cast `/Game/HTWContent/Blueprints/WIDGET_EnemyHealthBar` (`WidgetComponent.GetUserWidgetObject` (`self.HealthBar`))))
  (set `self.HealthBarWidget` _aswidget_enemy_health_bar)
  ;[1 1 1] Set MaxHealth and CurrentHealth of Widget
  (set `/Game/HTWContent/Blueprints/WIDGET_EnemyHealthBar.EnemyMaxHealth` (`self.StartingHealth`) _healthbarwidget)
  (set `/Game/HTWContent/Blueprints/WIDGET_EnemyHealthBar.EnemyCurrentHealth` _currenthealth _healthbarwidget)
  ;[1 1 1] Set Widget HealthProgress to be correct
  (`/Game/HTWContent/Blueprints/WIDGET_EnemyHealthBar.UpdateHealth` _healthbarwidget _currenthealth)
  (`/Game/HTWContent/Blueprints/WIDGET_EnemyHealthBar.SetColourOfHealthBar` _healthbarwidget (make `Color` 255 0 0 255)))

(event `self.ReceiveTick`
  (params (DeltaSeconds :type "Float (single-precision)"))
  (bind _staticmesh (`self.StaticMesh`))
  ;[1 1 1] If current Health is lesser than 0, destroy
  (if (<= (`self.CurrentHealth`) 0)
    (bind (_direction _time) (`Timeline|Timeline_0`)
      (:`Update`
        (`SceneComponent.K2_SetRelativeRotation` _staticmesh (`KismetMathLibrary.MakeRotator` 0.0 (* (`KismetMathLibrary.Sin` _time) -45.0)) true false)
        (`SceneComponent.K2_SetWorldLocation` _staticmesh (`SceneComponent.K2_GetComponentLocation` _staticmesh) true false)
        (`/Engine/EditorBlueprintResources/StandardMacros.DoOnce` false
          (:`Completed`
            (set `self.AIControllerClass` "/Script/Engine.Controller")
            (`GameplayStatics.PlaySoundAtLocation` "/Game/HTWContent/Audio/SW_BlueCannonDeath.SW_BlueCannonDeath" (0.0 0.0 0.0) (struct) 1.0 1.0 0.0 null null null)
            (`KismetSystemLibrary.Delay` 0.9)
            (bind _asbp_game_mode_htwcgame_mode (cast `/Game/HTWContent/Blueprints/BP_GameMode_HTWCGameMode` (`GameplayStatics.GetGameMode`)))
            (`/Game/HTWContent/Blueprints/BP_GameMode_HTWCGameMode.ReduceEnemies_Event` _asbp_game_mode_htwcgame_mode)
            (`self.K2_DestroyActor`)))))
    (else
      ;[1 1 1] Rotate HealthBar to face Player
      (`self.RotateHealthBarToPlayer`))))

(event `self.StaticMesh.OnComponentHit`
  (params (HitComponent :type "PrimitiveComponent Object Reference") (OtherActor :type "Actor Object Reference") (OtherComp :type "PrimitiveComponent Object Reference") (NormalImpulse :type "Vector Structure") (Hit :type "HitResult Structure (by ref)"))
  ;[1 1 1] Check if Enemy is Overlapped by Bullet
  (if (== (`GameplayStatics.GetObjectClass` OtherActor) "/Game/HTWContent/Blueprints/BP_Actor_Bullet.BP_Actor_Bullet_C")
    (bind _asbp_actor_bullet (cast `/Game/HTWContent/Blueprints/BP_Actor_Bullet` OtherActor))
    ;[1 1 1] Check if Bullet is same colour as Enemy
    (if (`|EnumEquality` (`/Game/HTWContent/Blueprints/BP_Actor_Bullet.BulletColor` _asbp_actor_bullet) (`self.EnemyColour`))
      ;[1 1 1] TakeDamage from the Bullet
      (`/Game/HTWContent/Blueprints/BP_Enemy.TakeDamage` 1)
      ;[1 1 1] Update HealthBar Widget
      (`/Game/HTWContent/Blueprints/WIDGET_EnemyHealthBar.UpdateHealth` (`self.HealthBarWidget`) (`self.CurrentHealth`)))
    (`self.K2_DestroyActor` _asbp_actor_bullet)))

(event `/Game/HTWContent/Blueprints/BP_Enemy.TakeDamage`
  (params (DamageTaken :type Integer))
  (set `self.CurrentHealth` (- (`self.CurrentHealth`) DamageTaken)))

(event `/Game/HTWContent/Blueprints/BP_Enemy.Attack`
  (`self.Fire Cannon`))

(fn `Fire Cannon`
  (bind _forward (`self.Forward`))
  (`|SpawnActorFromClass` "/Game/HTWContent/Blueprints/AI/AI_BlueCannon/BP_CannonBall.BP_CannonBall_C" (`KismetMathLibrary.MakeTransform` (+ (`SceneComponent.K2_GetComponentLocation` _forward) (* (`SceneComponent.GetForwardVector` _forward) (`self.Speed`))) (`SceneComponent.K2_GetComponentRotation` _forward)) "Undefined" "OverrideRootScale" null null))

(fn `RotateHealthBarToPlayer`
  (bind _healthbar (`self.HealthBar`))
  (`SceneComponent.K2_SetWorldRotation` _healthbar (`KismetMathLibrary.FindLookAtRotation` (`SceneComponent.K2_GetComponentLocation` _healthbar) (`PlayerCameraManager.GetCameraLocation` (`GameplayStatics.GetPlayerCameraManager` 0))) false false))

(fn `UserConstructionScript`)