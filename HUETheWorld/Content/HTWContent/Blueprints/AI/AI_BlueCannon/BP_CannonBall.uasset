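; BP_CannonBall is a projectile that flies along its arrow's forward vector every tick, playing a windup sound on spawn.
; After three seconds or on overlapping the player, which also stops that sound, it runs a shared explosion sequence with sound and particles.
; That sequence casts the overlap's actor to BP_Character_Player, damages it and triggers invulnerability unless already invulnerable, and destroys the cannonball only if the cast succeeds.
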(event `self.ReceiveBeginPlay`
  (bind _returnvalue (`SceneComponent.K2_GetComponentLocation` (`self.StaticMesh`)))
  (bind _returnvalue_2 (`GameplayStatics.SpawnSound2D` "/Game/HTWContent/Audio/SW_CannonWindup.SW_CannonWindup" 1.0 1.0 0.0 null))
  (set `self.SoundComponent` _returnvalue_2)
  (`KismetSystemLibrary.Delay` 3.0)
  (`GameplayStatics.SpawnSoundAtLocation` "/Game/HTWContent/Audio/SW_Explosion_1.SW_Explosion_1" _returnvalue (struct) 1.0 1.0 0.0 null null :!label _label)
  (`GameplayStatics.SpawnEmitterAtLocation` "/Game/StarterContent/Particles/P_Explosion.P_Explosion" _returnvalue)
  (bind _asbp_character_player (cast `/Game/HTWContent/Blueprints/BP_Character_Player` (stale `self.ReceiveActorBeginOverlap` OtherActor)))
  (if (not (`/Game/HTWContent/Blueprints/BP_Character_Player.isInvulnerable` _asbp_character_player))
    (`/Game/HTWContent/Blueprints/BP_Character_Player.TakeDamage` _asbp_character_player 1)
    (`GameplayStatics.PlaySoundAtLocation` "/Game/HTWContent/Audio/Character_Damaged.Character_Damaged" (`self.K2_GetActorLocation` _asbp_character_player) (struct) 1.0 1.0 0.0 null null null)
    (`/Game/HTWContent/Blueprints/BP_Character_Player.TriggerInvulnerabilityPeriod` _asbp_character_player))
  (`self.K2_DestroyActor`))

(event `self.ReceiveActorBeginOverlap`
  (params (OtherActor :type "Actor Object Reference"))
  (if (== OtherActor (`GameplayStatics.GetPlayerCharacter` 0))
    (`AudioComponent.Stop` (`self.SoundComponent`))
    (goto _label)))

(event `self.ReceiveTick`
  (params (DeltaSeconds :type "Float (single-precision)"))
  (`self.K2_AddActorWorldOffset` (* (`SceneComponent.GetForwardVector` (`self.Arrow`)) 50.0)))

(fn `UserConstructionScript`)