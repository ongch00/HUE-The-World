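; BP_RedSlime is a slime enemy that only takes damage from bullets matching its colour.
; Static mesh hits from BP_Actor_Bullet compare bullet and enemy colour, then subtract fixed damage from health and print the result for debugging.
; Health is set from a starting value on BeginPlay, and Tick destroys the actor once it reaches zero.
; Random colour selection exists but is disconnected, so the colour stays fixed.
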(event `self.ReceiveBeginPlay`
  ;[1 1 1] Set current health of enemy
  (set `self.CurrentHealth` (`self.StartingHealth`)))

(event `self.ReceiveTick`
  (params (DeltaSeconds :type "Float (single-precision)"))
  ;[1 1 1] If current Health is lesser than 0, destroy
  (if (<= (`self.CurrentHealth`) 0)
    (`self.K2_DestroyActor`)))

(event `self.StaticMesh.OnComponentHit`
  (params (HitComponent :type "PrimitiveComponent Object Reference") (OtherActor :type "Actor Object Reference") (OtherComp :type "PrimitiveComponent Object Reference") (NormalImpulse :type "Vector Structure") (Hit :type "HitResult Structure (by ref)"))
  ;[1 1 1] Check if Enemy is Overlapped by Bullet
  (if (== (`GameplayStatics.GetObjectClass` OtherActor) "/Game/HTWContent/Blueprints/BP_Actor_Bullet.BP_Actor_Bullet_C")
    (bind _asbp_actor_bullet (cast `/Game/HTWContent/Blueprints/BP_Actor_Bullet` OtherActor))
    ;[1 1 1] Check if Bullet is same colour as Enemy
    (if (`|EnumEquality` (`/Game/HTWContent/Blueprints/BP_Actor_Bullet.BulletColor` _asbp_actor_bullet) (`self.EnemyColour`))
      (`/Game/HTWContent/Blueprints/BP_Enemy.TakeDamage` 2)
      (`KismetSystemLibrary.PrintString` (`KismetStringLibrary.Conv_IntToString` (`self.CurrentHealth`))))))

(event `/Game/HTWContent/Blueprints/BP_Enemy.TakeDamage`
  (params (DamageTaken :type Integer))
  (set `self.CurrentHealth` (- (`self.CurrentHealth`) DamageTaken)))

(fn `UserConstructionScript`)