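; Bullet actor with a paint color of red, blue or yellow.
; SetMaterial applies the matching paint material to BulletModel based on BulletColor, though nothing in this graph calls it.
; On hit, the bullet destroys itself unless the other actor is a BP_Enemy, in which case it does nothing here.
; Tick is empty, and the forward-offset movement using BulletSpeed is disconnected, so it never runs.
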(event `self.ReceiveTick`
  (params (DeltaSeconds :type "Float (single-precision)")))

(event `self.BulletModel.OnComponentHit`
  (params (HitComponent :type "PrimitiveComponent Object Reference") (OtherActor :type "Actor Object Reference") (OtherComp :type "PrimitiveComponent Object Reference") (NormalImpulse :type "Vector Structure") (Hit :type "HitResult Structure (by ref)"))
  (cast `/Game/HTWContent/Blueprints/BP_Enemy` OtherActor
    (:`CastFailed`
      (`self.K2_DestroyActor`))))

(fn `SetMaterial`
  (bind _bulletmodel (`self.BulletModel`))
  (switch `/Game/HTWContent/Blueprints/BP_Enum_Colours` (`self.BulletColor`)
    (:`NewEnumerator0`
      (`PrimitiveComponent.SetMaterial` _bulletmodel 0 "/Game/HTWContent/Meshes/Forest/M_RedPaint.M_RedPaint"))
    (:`NewEnumerator1`
      (`PrimitiveComponent.SetMaterial` _bulletmodel 0 "/Game/HTWContent/Meshes/Forest/M_BluePaint.M_BluePaint"))
    (:`NewEnumerator2`
      (`PrimitiveComponent.SetMaterial` _bulletmodel 0 "/Game/HTWContent/Meshes/Forest/M_YellowPaint.M_YellowPaint")))
  (return))

(fn `UserConstructionScript`)