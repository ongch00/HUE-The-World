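; Game mode that tracks the remaining enemies in a level and reveals the portal once all are gone.
; BeginPlay counts actors via the BP_Enemy interface, hides the portal with collision off, and applies the MI_City material to every static mesh actor.
; ReduceEnemies_Event decrements the count; at zero it restores the portal and plays a timeline driving the Fade parameter in the LevelMPC material parameter collection.
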(event `self.ReceiveBeginPlay`
  (bind _outactors (`GameplayStatics.GetAllActorsWithInterface` "/Game/HTWContent/Blueprints/BP_Enemy.BP_Enemy_C"))
  (set `self.EnemyCount` (`KismetArrayLibrary.Array_Length` _outactors))
  (bind _returnvalue (`GameplayStatics.GetActorOfClass` "/Game/HTWContent/Blueprints/BP_Portal.BP_Portal_C"))
  (bind _output_get (set `self.Portal` _returnvalue))
  (`self.SetActorHiddenInGame` _output_get true)
  (`self.SetActorEnableCollision` _output_get false)
  (bind _outactors_2 (`GameplayStatics.GetAllActorsOfClass` "/Script/Engine.StaticMeshActor"))
  (bind _output_get_2 (set `self.StaticMeshes` _outactors_2))
  (for _array_element _output_get_2
    (`PrimitiveComponent.SetMaterial` (`StaticMeshActor.StaticMeshComponent` _array_element) 0 "/Game/HTWContent/Materials/MI_City.MI_City")))

(event `ReduceEnemies_Event`
  (bind _enemycount (`self.EnemyCount`))
  (bind _portal (`self.Portal`))
  (`/Engine/EditorBlueprintResources/StandardMacros.DecrementInt` _enemycount
    (:`  `
      (if (<= _enemycount 0)
        (`self.SetActorHiddenInGame` _portal false)
        (`self.SetActorEnableCollision` _portal true)
        (bind (_direction _newtrack_0) (`Timeline|Timeline_0`)
          (:`Update`
            (`KismetMaterialLibrary.SetScalarParameterValue` "/Game/HTWContent/Materials/LevelMPC.LevelMPC" "Fade" _newtrack_0)))))))

(fn `UserConstructionScript`)