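; BP_Actor_Enemy is an enemy actor that is destroyed when hit by a bullet of matching colour.
; On BeginPlay it sets its EnemyColour to a fixed value for debugging; the random pick from PossibleEnemyColours is disconnected.
; When its Enemy component overlaps a BP_Actor_Bullet, it compares BulletColor to EnemyColour and destroys itself on a match, leaving the bullet untouched.
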(event `self.ReceiveBeginPlay`
  ;[1 1 1] Set Random Enemy Colour (currently fixed for debugging)
  (set `self.EnemyColour` "NewEnumerator0"))

(event `self.Enemy.OnComponentBeginOverlap`
  (params (OverlappedComponent :type "PrimitiveComponent Object Reference") (OtherActor :type "Actor Object Reference") (OtherComp :type "PrimitiveComponent Object Reference") (OtherBodyIndex :type Integer) (bFromSweep :type Boolean) (SweepResult :type "HitResult Structure (by ref)"))
  ;[1 1 1] Check if Enemy is Overlapped by Bullet
  (if (== (`GameplayStatics.GetObjectClass` OtherActor) "/Game/HTWContent/Blueprints/BP_Actor_Bullet.BP_Actor_Bullet_C")
    (bind _asbp_actor_bullet (cast `/Game/HTWContent/Blueprints/BP_Actor_Bullet` OtherActor))
    ;[1 1 1] Check if Bullet is same colour as Enemy
    (if (`|EnumEquality` (`/Game/HTWContent/Blueprints/BP_Actor_Bullet.BulletColor` _asbp_actor_bullet) (`self.EnemyColour`))
      (`self.K2_DestroyActor`))))

(fn `UserConstructionScript`)