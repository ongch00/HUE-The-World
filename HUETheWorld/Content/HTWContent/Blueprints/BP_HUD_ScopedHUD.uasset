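; HUD class that shows the health bar, a crosshair and the ammo, reload, restart and pause notification widgets.
; BeginPlay adds the health bar widget, and DrawHUD draws a small dashed-circle crosshair at screen center.
; Show/hide functions create, store and remove each notification; HideAmmoNotification also clears the reload-only one if no ammo notice exists.
; Pause notification functions also pause and unpause the game, and the restart notice refreshes its levels.
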(event `self.ReceiveBeginPlay`
  (bind _returnvalue (`|CreateWidget` "/Game/HTWContent/Blueprints/BP_HealthBar.BP_HealthBar_C"))
  (`UserWidget.AddToViewport` _returnvalue 0))

(event `self.ReceiveDrawHUD`
  (params (SizeX :type Integer) (SizeY :type Integer))
  ;[1 1 1] Draw CrossHair
  (`self.DrawTexture` "/Game/HTWContent/Textures/T_Circle_Dashed.T_Circle_Dashed" (`KismetMathLibrary.Conv_IntToDouble` (/ SizeX 2)) (`KismetMathLibrary.Conv_IntToDouble` (/ SizeY 2)) 10.0 10.0 0.0 0.0 0.0 0.0 (struct :`R` 1.0 :`B` 0.375613 :`A` 1.0) "BLEND_Masked"))

(fn `HideAmmoNotification`
  (if (`KismetSystemLibrary.IsValid` (`self.AmmoNotificationWidget`))
    (`Widget.RemoveFromParent` (`self.AmmoNotificationWidget`))
    (set `self.AmmoNotificationWidget` null)
    (elif (`KismetSystemLibrary.IsValid` (`self.ReloadOnlyNotificationWidget`))
      (`Widget.RemoveFromParent` (`self.ReloadOnlyNotificationWidget`))
      (set `self.ReloadOnlyNotificationWidget` null))))

(fn `HidePauseNotification`
  (`Widget.RemoveFromParent` (`self.PauseNotificationWidget`))
  (`GameplayStatics.SetGamePaused` false))

(fn `HideRestartNotification`
  (`Widget.RemoveFromParent` (`self.RestartNotificationWidget`)))

(fn `ShowAmmoNotification`
  (bind _returnvalue (`|CreateWidget` "/Game/HTWContent/Blueprints/WIDGET_AmmoNotif.WIDGET_AmmoNotif_C"))
  (`UserWidget.AddToViewport` _returnvalue 0)
  (set `self.AmmoNotificationWidget` _returnvalue))

(fn `ShowPauseNotification`
  (bind _returnvalue (`|CreateWidget` "/Game/HTWContent/Blueprints/WIDGET_PauseNotif.WIDGET_PauseNotif_C"))
  (`UserWidget.AddToViewport` _returnvalue 0)
  (set `self.PauseNotificationWidget` _returnvalue)
  (`GameplayStatics.SetGamePaused` true))

(fn `ShowReloadOnlyNotification`
  (bind _returnvalue (`|CreateWidget` "/Game/HTWContent/Blueprints/WIDGET_ReloadOnlyNotif.WIDGET_ReloadOnlyNotif_C"))
  (`UserWidget.AddToViewport` _returnvalue 0)
  (set `self.ReloadOnlyNotificationWidget` _returnvalue))

(fn `ShowRestartNotification`
  (bind _returnvalue (`|CreateWidget` "/Game/HTWContent/Blueprints/WIDGET_RestartNotif.WIDGET_RestartNotif_C"))
  (`UserWidget.AddToViewport` _returnvalue 0)
  (bind _output_get (set `self.RestartNotificationWidget` _returnvalue))
  (`/Game/HTWContent/Blueprints/WIDGET_RestartNotif.Update Levels` _output_get)
  (`/Game/HTWContent/Blueprints/WIDGET_RestartNotif.Update Levels` _returnvalue))

(fn `UserConstructionScript`)